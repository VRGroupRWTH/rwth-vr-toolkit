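; Test actor in the grabbing component folder that gives visual feedback for hover and click interaction on a static mesh.
; Events from its HoverBehaviour and ClickBehaviour components swap the material in slot 0 to show hovered, clicked or idle state.
; Ending a click always restores the hover material, and only ending a hover applies the ball material.
; It contains no grab logic; the construction script and NewFunction are empty.
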(event `self.HoverBehaviour.OnHoverStartEvent`
  (params (TriggeredComponent :type "SceneComponent Object Reference") (Hit :type "HitResult Structure"))
  (`PrimitiveComponent.SetMaterial` (`self.StaticMesh`) 0 "/Engine/VREditor/BasicMeshes/MI_Cube_01.MI_Cube_01"))

(event `self.HoverBehaviour.OnHoverEndEvent`
  (params (TriggeredComponent :type "SceneComponent Object Reference"))
  (`PrimitiveComponent.SetMaterial` (`self.StaticMesh`) 0 "/Engine/VREditor/BasicMeshes/MI_Ball_01.MI_Ball_01"))

(event `self.ClickBehaviour.OnClickStartEvent`
  (params (TriggeredComponent :type "SceneComponent Object Reference") (Value :type "InputActionValue Structure (by ref)"))
  (`PrimitiveComponent.SetMaterial` (`self.StaticMesh`) 0 "/Engine/VREditor/BasicMeshes/MI_Cube_03.MI_Cube_03"))

(event `self.ClickBehaviour.OnClickEndEvent`
  (params (TriggeredComponent :type "SceneComponent Object Reference") (Value :type "InputActionValue Structure (by ref)"))
  (`PrimitiveComponent.SetMaterial` (`self.StaticMesh`) 0 "/Engine/VREditor/BasicMeshes/MI_Cube_01.MI_Cube_01"))

(fn `NewFunction`)

(fn `UserConstructionScript`)