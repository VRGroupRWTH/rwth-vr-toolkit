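; BP_CaveSetup is an RWTH VR Cluster actor that holds the Aixcave child actor and keeps it only in room-mounted display mode.
; When not in room-mounted mode, the construction script turns off the component's visibility, propagating to children, though it sets the child actor's hidden-in-game flag to false.
; In that same case, BeginPlay destroys the child actor.
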(event `self.ReceiveBeginPlay`
  (if (not (`RWTHVRUtilities.IsRoomMountedMode`))
    (`self.K2_DestroyActor` (`ChildActorComponent.ChildActor` (`self.aixcave`)))))

(fn `UserConstructionScript`
  (if (not (`RWTHVRUtilities.IsRoomMountedMode`))
    (`self.SetActorHiddenInGame` (`ChildActorComponent.ChildActor` (`self.aixcave`)) false)
    (`SceneComponent.SetVisibility` (`self.aixcave`) false true)))