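; BP_RE_1_2 is a replication example actor that shows how execution branches on network authority.
; On BeginPlay, a Switch Has Authority node sets a text render to read either "Authority" or "Client".
; Only on the client, it also casts the child actor to BP_locomotive and raises the play rate in that locomotive's animation instance, so the change is made locally.
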(event `self.ReceiveBeginPlay`
  (bind _textrender (`self.TextRender`))
  (`parent.ReceiveBeginPlay`)
  (`/Engine/EditorBlueprintResources/ActorMacros.Switch Has Authority` ; Switch on whether the machine executing this blueprint is a network authority or not
    (:`Authority`
      (`TextRenderComponent.K2_SetText` _textrender "Authority"))
    (:`Remote`
      (`TextRenderComponent.K2_SetText` _textrender "Client")
      (bind _asbp_locomotive (cast `/RWTHVRToolkit/ReplicationExamples/Blueprints/BP_locomotive` (`ChildActorComponent.ChildActor` (`self.BP_loc_replication`))))
      (bind _asbp_locomotive_animation (cast `/RWTHVRToolkit/ReplicationExamples/Models/BP_locomotiveAnimation` (`SkeletalMeshComponent.GetAnimInstance` (`/RWTHVRToolkit/ReplicationExamples/Blueprints/BP_locomotive.locomotive` _asbp_locomotive))))
      (set `/RWTHVRToolkit/ReplicationExamples/Models/BP_locomotiveAnimation.PlayRate` 20.0 _asbp_locomotive_animation))))

(fn `UserConstructionScript`
  (`parent.UserConstructionScript`))