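; Replication example actor that demonstrates a RepNotify variable by stopping and starting a locomotive animation.
; On authority, a loop started at BeginPlay alternates PlayRate between 0 and 1 after random one-to-two-second delays.
; OnRep_PlayRate passes the value to the animation Blueprint of the BP_locomotive held in the BPLocReplication child actor component.
; The Repeat event re-enters the BeginPlay chain, including its parent call.
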(event `self.ReceiveBeginPlay`
  (`parent.ReceiveBeginPlay` :!label _label)
  (`/Engine/EditorBlueprintResources/ActorMacros.Switch Has Authority`
    (:`Authority`
      (`KismetSystemLibrary.Delay` (`KismetMathLibrary.RandomFloatInRange` 1.0 2.0))
      (set `self.PlayRate` 0.0)
      (`KismetSystemLibrary.Delay` (`KismetMathLibrary.RandomFloatInRange` 1.0 2.0))
      (set `self.PlayRate` 1.0)
      (`self.Repeat`))))

(event `Repeat`
  (goto _label))

(fn `OnRep_PlayRate`
  (bind _asbp_locomotive (cast `/RWTHVRToolkit/ReplicationExamples/Blueprints/BP_locomotive` (`ChildActorComponent.ChildActor` (`self.BP_loc_replication`))))
  (bind _asbp_locomotive_animation (cast `/RWTHVRToolkit/ReplicationExamples/Models/BP_locomotiveAnimation` (`SkeletalMeshComponent.GetAnimInstance` (`/RWTHVRToolkit/ReplicationExamples/Blueprints/BP_locomotive.locomotive` _asbp_locomotive))))
  (set `/RWTHVRToolkit/ReplicationExamples/Models/BP_locomotiveAnimation.PlayRate` (`self.PlayRate`) _asbp_locomotive_animation))

(fn `UserConstructionScript`
  (`parent.UserConstructionScript`))