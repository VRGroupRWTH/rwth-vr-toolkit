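; Replication example 1.5: an actor that plays a locomotive's animation while something overlaps its capsule.
; BeginPlay pauses the animation of the child-actor locomotive by setting its anim instance PlayRate to zero.
; Capsule begin and end overlaps are handled only on the authority, which calls ToggleAnimation, grouped under Multicast Events, to switch PlayRate between running and paused.
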(event `self.ReceiveBeginPlay`
  (bind _asbp_locomotive (cast `/RWTHVRToolkit/ReplicationExamples/Blueprints/BP_locomotive` (`ChildActorComponent.ChildActor` (`self.BP_loc_replication`))))
  (bind _asbp_locomotive_animation (cast `/RWTHVRToolkit/ReplicationExamples/Models/BP_locomotiveAnimation` (`SkeletalMeshComponent.GetAnimInstance` (`/RWTHVRToolkit/ReplicationExamples/Blueprints/BP_locomotive.locomotive` _asbp_locomotive))))
  (set `/RWTHVRToolkit/ReplicationExamples/Models/BP_locomotiveAnimation.PlayRate` 0.0 _asbp_locomotive_animation))

(event `self.Capsule.OnComponentBeginOverlap`
  (params (OverlappedComponent :type "PrimitiveComponent Object Reference") (OtherActor :type "Actor Object Reference") (OtherComp :type "PrimitiveComponent Object Reference") (OtherBodyIndex :type Integer) (bFromSweep :type Boolean) (SweepResult :type "HitResult Structure (by ref)"))
  (`/Engine/EditorBlueprintResources/ActorMacros.Switch Has Authority`
    (:`Authority`
      (`self.ToggleAnimation` true))))

(event `self.Capsule.OnComponentEndOverlap`
  (params (OverlappedComponent :type "PrimitiveComponent Object Reference") (OtherActor :type "Actor Object Reference") (OtherComp :type "PrimitiveComponent Object Reference") (OtherBodyIndex :type Integer))
  (`/Engine/EditorBlueprintResources/ActorMacros.Switch Has Authority`
    (:`Authority`
      (`self.ToggleAnimation` false))))

(event `ToggleAnimation`
  (params (StartAnimation :type Boolean))
  (bind _asbp_locomotive (cast `/RWTHVRToolkit/ReplicationExamples/Blueprints/BP_locomotive` (`ChildActorComponent.ChildActor` (`self.BP_loc_replication`))))
  (bind _asbp_locomotive_animation (cast `/RWTHVRToolkit/ReplicationExamples/Models/BP_locomotiveAnimation` (`SkeletalMeshComponent.GetAnimInstance` (`/RWTHVRToolkit/ReplicationExamples/Blueprints/BP_locomotive.locomotive` _asbp_locomotive))))
  (if StartAnimation
    (set `/RWTHVRToolkit/ReplicationExamples/Models/BP_locomotiveAnimation.PlayRate` 1.0 _asbp_locomotive_animation)
    (else
      (set `/RWTHVRToolkit/ReplicationExamples/Models/BP_locomotiveAnimation.PlayRate` 0.0 _asbp_locomotive_animation))))

(fn `UserConstructionScript`
  (`parent.UserConstructionScript`))