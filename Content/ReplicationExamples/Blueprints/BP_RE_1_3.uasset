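; Replication example that contrasts a replicated and a non-replicated variable, judging by names, through the animation play rates of two locomotives.
; On authority only, a looping timer steps both rates from the replicated value and flips the step direction at the min and max limits.
; Tick has no authority check and pushes each rate into its child locomotive's animation Blueprint and a text display, exposing any server-client difference.
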(event EventBeginPlay
  (|CallParentFunction)
  (Networking|SwitchHasAuthority
    (:Authority
      (Utilities|Time|SetTimerbyFunctionName 0 "UpdatePlayRates" (Variables|Default|GetPlayRate_Timer) true))))

(event EventTick
  (params (DeltaSeconds :type Float%20%28single-precision%29))
  (bind _playrate_rep (Variables|Default|GetPlayRate_Rep))
  (bind _playrate_norep (Variables|Default|GetPlayRate_NoRep))
  (|CallParentFunction DeltaSeconds)
  (bind _asbp_locomotive (Utilities|Casting|CastToBP_locomotive (Variables|/Script/Engine.ChildActorComponent|GetChildActor (Variables|Default|GetBP_loc_VarRep))))
  (CallFunction|SetLocomotivePlayrate _asbp_locomotive _playrate_rep)
  (Rendering|Components|TextRender|SetText (Variables|Default|GetRepReplayRate) (Utilities|Text|ToText(String) (Class|KismetStringLibrary|BuildStringDouble "" "PlayRate: " _playrate_rep)))
  (bind _asbp_locomotive_2 (Utilities|Casting|CastToBP_locomotive (Variables|/Script/Engine.ChildActorComponent|GetChildActor (Variables|Default|GetBP_loc_NoVarRep))))
  (CallFunction|SetLocomotivePlayrate _asbp_locomotive_2 _playrate_norep)
  (Rendering|Components|TextRender|SetText (Variables|Default|GetNoRepReplayRate) (Utilities|Text|ToText(String) (Class|KismetStringLibrary|BuildStringDouble "" "PlayRate: " _playrate_norep))))

(fn ConstructionScript
  (|CallParentFunction))

(fn SetLocomotivePlayrate
  (params (locomotive :type BP%20Locomotive%20Object%20Reference) (NewSpeed :type Float%20%28double-precision%29))
  (bind _asbp_locomotive_animation (Utilities|Casting|CastToBP_locomotiveAnimation (Components|SkeletalMesh|GetAnimInstance (Variables|/RWTHVRToolkit/ReplicationExamples/Blueprints/BP_locomotive.BP_locomotive_C|Getlocomotive locomotive))))
  (Variables|/RWTHVRToolkit/ReplicationExamples/Models/BP_locomotiveAnimation.BP_locomotiveAnimation_C|SetPlayRate _asbp_locomotive_animation NewSpeed))

(fn UpdatePlayRates
  (Variables|Default|SetPlayRate_NoRep (|(PlayRate+({23C983A3-4F59-D834-B0AF-3681B7CDCF37}*{6D207F80-47B3-ADEE-F574-E19BF15B22B3})) (stale _output_get)))
  (bind _output_get (Variables|Default|SetPlayRate_Rep (|(PlayRate+({23C983A3-4F59-D834-B0AF-3681B7CDCF37}*{6D207F80-47B3-ADEE-F574-E19BF15B22B3})) (stale _output_get))))
  (if (or (<= (|(PlayRate+({23C983A3-4F59-D834-B0AF-3681B7CDCF37}*{6D207F80-47B3-ADEE-F574-E19BF15B22B3})) _output_get) (Variables|Default|GetPlayRate_Min)) (>= (|(PlayRate+({23C983A3-4F59-D834-B0AF-3681B7CDCF37}*{6D207F80-47B3-ADEE-F574-E19BF15B22B3})) _output_get) (Variables|Default|GetPlayRate_Max)))
    (Variables|Default|SetModifier (* (Variables|Default|GetModifier) -1))))