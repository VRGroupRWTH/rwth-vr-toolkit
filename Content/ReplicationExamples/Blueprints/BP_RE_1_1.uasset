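; BP_RE_1_1 is a replication example actor that spawns a non-replicated actor and a replicated one, to contrast how each appears across the network.
; On BeginPlay a Switch Has Authority gate lets only the authority spawn BP_loc_NoReplication and BP_loc_replication.
; Each spawns at the transform of its own target reference, NoRepTarget or RepTarget.
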(event `self.ReceiveBeginPlay`
  (`parent.ReceiveBeginPlay`)
  (`/Engine/EditorBlueprintResources/ActorMacros.Switch Has Authority`
    (:`Authority`
      (`|SpawnActorFromClass` "/RWTHVRToolkit/ReplicationExamples/Blueprints/BP_loc_NoReplication.BP_loc_NoReplication_C" (`self.GetTransform` (`self.NoRepTarget`)) "Undefined" "MultiplyWithRoot" null null)
      (`|SpawnActorFromClass` "/RWTHVRToolkit/ReplicationExamples/Blueprints/BP_loc_replication.BP_loc_replication_C" (`self.GetTransform` (`self.RepTarget`)) "Undefined" "MultiplyWithRoot" null null))))

(fn `UserConstructionScript`
  (`parent.UserConstructionScript`))